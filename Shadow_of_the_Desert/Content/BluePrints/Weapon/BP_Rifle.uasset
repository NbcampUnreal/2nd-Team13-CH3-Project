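; BP_Rifle is a rifle weapon Blueprint whose graph holds only a scripted fire-and-reload sequence.
; On BeginPlay it chains Delay nodes to call Attack at varying intervals, calls Reload, then fires twice back to back after a pause.
; Attack and Reload are not defined in these graphs, and the construction script is empty.
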(event `self.ReceiveBeginPlay`
  (`KismetSystemLibrary.Delay` 0.2)
  (`self.Attack`)
  (`KismetSystemLibrary.Delay` 0.2)
  (`self.Attack`)
  (`KismetSystemLibrary.Delay` 1.0)
  (`self.Attack`)
  (`KismetSystemLibrary.Delay` 1.0)
  (`self.Attack`)
  (`self.Reload`)
  (`KismetSystemLibrary.Delay` 2.0)
  (`self.Attack`)
  (`self.Attack`))

(fn `UserConstructionScript`)