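; Behavior tree task that sends an enemy AI along the waypoints of a BP_PatrolPath.
; It reads the path and current index from the blackboard and runs AIMoveTo toward that waypoint actor.
; On move success it binds a handler to the controller's ReceiveMoveCompleted, then finishes the task as failed.
; That handler advances the blackboard index, wrapping at the end of the path, without checking the move result.
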(event `self.ReceiveExecuteAI`
  (params (OwnerController :type "AIController Object Reference") (ControlledPawn :type "Pawn Object Reference"))
  (bind _asbp_patrol_path (cast `/Game/BluePrints/Enemy/BP_PatrolPath` (`BTFunctionLibrary.GetBlackboardValueAsObject` (`self.patrolPathKey`))))
  (`|AIMoveTo` ControlledPawn (0.0 0.0 0.0) (`|GetArrayItem` (`PatrolPath.wayPoints` _asbp_patrol_path) (`BTFunctionLibrary.GetBlackboardValueAsInt` (`self.currentWaypointIdxKey`)))
    (:`OnSuccess`
      (add `AIController.ReceiveMoveCompleted` OwnerController (delegate `MoveCompletedEvent`))
      (`self.FinishExecute` false))))

(event `MoveCompletedEvent`
  (params (RequestID :type "AIRequestID Structure") (Result :type "EPathFollowingResult Enum" :default "Success"))
  (bind _currentwaypointidxkey (`self.currentWaypointIdxKey`))
  (`BTFunctionLibrary.SetBlackboardValueAsInt` _currentwaypointidxkey (mod (+ (`BTFunctionLibrary.GetBlackboardValueAsInt` _currentwaypointidxkey) 1) (`KismetArrayLibrary.Array_Length` (`PatrolPath.wayPoints` (stale `self.ReceiveExecuteAI` _asbp_patrol_path))))))