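; BP_EnemyCatus is an enemy Blueprint that reports player sightings or losses from its AIPerception component to its AI.
; On each target perception update, it responds only if the actor is a TestCharacter and its controller is a BP_EnemyAIController.
; A successful sense sets the detected flag and target actor on that controller's Blackboard, while a failed one clears both.
; BeginPlay, Tick, overlap and construction logic are empty.
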(event `self.AIPerception.OnTargetPerceptionUpdated`
  (params (Actor :type "Actor Object Reference") (Stimulus :type "AIStimulus Structure"))
  (bind _astest_character (cast `/Game/BluePrints/TestCharacter` Actor))
  (bind _asbp_enemy_aicontroller (cast `/Game/BluePrints/Enemy/TestAsset/BP_EnemyAIController` (`self.GetController`)))
  (if Stimulus_bSuccessfullySensed
    (bind _returnvalue (`AIBlueprintHelperLibrary.GetBlackboard` _asbp_enemy_aicontroller))
    (`BlackboardComponent.SetValueAsBool` _returnvalue (`self.playerDetectedKey`) true)
    (`BlackboardComponent.SetValueAsObject` _returnvalue (`self.targetActorKey`) _astest_character)
    (else
      (bind _returnvalue_2 (`AIBlueprintHelperLibrary.GetBlackboard` _asbp_enemy_aicontroller))
      (`BlackboardComponent.SetValueAsBool` _returnvalue_2 (`self.playerDetectedKey`) false)
      (`BlackboardComponent.SetValueAsObject` _returnvalue_2 (`self.targetActorKey`) null))))

(fn `UserConstructionScript`)