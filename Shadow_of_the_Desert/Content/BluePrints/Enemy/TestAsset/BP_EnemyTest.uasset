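; BP_EnemyTest is a test enemy Blueprint that assigns itself a patrol route at BeginPlay.
; It scans actors tagged "Route", printing "Hello" if none exist, and casts selected ones to BP_PatrolRoute to set PatrolRoute.
; The comparison keeps increasing distances, so it favors the farthest route despite the NearRoute naming.
; An alternative sphere-overlap search sits unconnected and never runs.
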(event `self.ReceiveBeginPlay`
  ; Tag
  (`parent.ReceiveBeginPlay`)
  (bind _outactors (`GameplayStatics.GetAllActorsWithTag` "Route"))
  (bind _output_get (set `self.Out Actors_0` _outactors))
  (if (== 0 (`KismetArrayLibrary.Array_Length` _output_get))
    (`KismetSystemLibrary.PrintText` "Hello")
    (else
      (for _array_element (`self.Out Actors_0`)
        (bind _returnvalue (`KismetMathLibrary.Vector_Distance` (`self.K2_GetActorLocation`) (`self.K2_GetActorLocation` _array_element)))
        (if (< (`self.CurrDist_0`) _returnvalue)
          (set `self.CurrDist_0` _returnvalue)
          (bind _output_get_2 (set `self.NearRoute_0` _array_element))
          (bind _asbp_patrol_route (cast `/Game/BluePrints/Enemy/BP_PatrolRoute` _output_get_2))
          (set `self.patrolRoute` _asbp_patrol_route))))))

(fn `UserConstructionScript`
  (`parent.UserConstructionScript`))