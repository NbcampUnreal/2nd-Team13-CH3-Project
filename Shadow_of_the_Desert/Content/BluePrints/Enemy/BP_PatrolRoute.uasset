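; BP_PatrolRoute is an enemy patrol path actor that supplies waypoints from a spline.
; IncrementPatrolRoute steps PatrolIdx by Direction, flipping Direction at the last and first spline points for back-and-forth patrolling.
; GetSplinePointAsWorldPosition returns the world location of the current spline point.
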(event `IncrementPatrolRoute`
  (bind _output_get (set `self.patrolIdx` (+ (`self.patrolIdx`) (`self.direction`))))
  (if (== _output_get (- (`SplineComponent.GetNumberOfSplinePoints` (`self.PatrolRoute`)) 1))
    (set `self.direction` -1)
    (elif (== (`self.patrolIdx`) 0)
      (set `self.direction` 1))))

(fn `GetSplinePointAsWorldPosition`
  (returns (Location :type "Vector Structure"))
  (return (`SplineComponent.GetLocationAtSplinePoint` (`self.PatrolRoute`) (`self.patrolIdx`) "World")))

(fn `UserConstructionScript`)