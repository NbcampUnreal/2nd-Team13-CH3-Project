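; Base enemy character Blueprint providing shared chase, attack, patrol-route and movement-speed behavior.
; ChasePlayerBase uses AI MoveTo toward player 0, calls AttackBase on success, then re-calls itself after a short delay; failed moves end the loop.
; AttackBase plays a one-shot animation directly on the mesh, leaving montage and EnemyAttack nodes unconnected.
; GetPatrolRoute exposes the route, and SetMovementSpeed maps an idle/walk/run state to max walk speed.
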(event `self.ReceiveBeginPlay`)

(event `ChasePlayerBase`
  (`|AIMoveTo` self (0.0 0.0 0.0) (`GameplayStatics.GetPlayerCharacter` 0) 150.0
    (:`OnSuccess`
      (`self.AttackBase`)
      (`KismetSystemLibrary.Delay` 1.0)
      (`self.ChasePlayerBase`))))

(event `AttackBase`
  (`SkeletalMeshComponent.PlayAnimation` (`self.Mesh`) (`self.attackAnim`) false))

(fn `GetPatrolRoute`
  (returns (patrolRoute :type "/Game/BluePrints/Enemy/BP_PatrolRoute Object Reference"))
  (return (`self.patrolRoute`)))

(fn `SetMovementSpeed`
  (params (Speed :type "/Game/BluePrints/Enemy/Enum_EnemySpeed Enum" :default "NewEnumerator0"))
  (returns (SpeedValue :type "Float (double-precision)"))
  (bind _output_get (set `CharacterMovementComponent.MaxWalkSpeed` (select `/Game/BluePrints/Enemy/Enum_EnemySpeed` Speed :`NewEnumerator1` 500.0 :`NewEnumerator2` 1500.0 :!type "Float (single-precision)") (`self.CharacterMovement`)))
  (return _output_get))

(fn `UserConstructionScript`)