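; Base enemy AI controller that runs BT_EnemyBase on possess and drives its Blackboard state, starting at Idle.
; Perception updates are checked per sense through CanSenseActor, which matches stimuli by sense class.
; While Idle or Investigating, seeing the player sets Attacking with a target, and hearing sets Investigating with a point of interest.
; Damage sensing triggers nothing; SetStateAsOnDamaged writes Hit to a separate key but is uncalled here.
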(event `self.ReceivePossess`
  (params (PossessedPawn :type "Pawn Object Reference"))
  (`self.RunBehaviorTree` "/Game/BluePrints/Enemy/BT_EnemyBase.BT_EnemyBase")
  (`self.SetStateAsIdle`))

(event `self.AIPerception.OnPerceptionUpdated`
  (params (UpdatedActors :type "Array of Actor Object Reference (by ref)"))
  (for _array_element UpdatedActors
    (`|ExecutionSequence`
      (:`then_0`
        (bind _sensed (`self.CanSenseActor` _array_element "NewEnumerator1"))
        (if _sensed
          (`self.HandleSenseSight` _array_element)))
      (:`then_1`
        (bind (_sensed_2 _stimulus) (`self.CanSenseActor` _array_element "NewEnumerator2"))
        (if _sensed_2
          (`self.HandleSenseSound` (`.StimulusLocation` (break `AIStimulus` _stimulus)))))
      (:`then_2`
        (bind _sensed_3 (`self.CanSenseActor` _array_element "NewEnumerator3"))
        (if _sensed_3
          _)))))

(fn `CanSenseActor`
  (params (Actor :type "Actor Object Reference") (Sense :type "/Game/BluePrints/Enemy/Enum_AiSense Enum" :default "NewEnumerator0"))
  (returns (Sensed :type Boolean) (Stimulus :type "AIStimulus Structure"))
  (bind _info (`AIPerceptionComponent.GetActorsPerception` (`self.AIPerception`) Actor))
  (for _array_element (`.LastSensedStimuli` (break `ActorPerceptionBlueprintInfo` _info))
    (bind _returnvalue (`AIPerceptionSystem.GetSenseClassForStimulus` _array_element))
    (if (== _returnvalue (select `/Game/BluePrints/Enemy/Enum_AiSense` Sense :`NewEnumerator1` "/Script/AIModule.AISense_Sight" :`NewEnumerator2` "/Script/AIModule.AISense_Hearing" :`NewEnumerator3` "/Script/AIModule.AISense_Damage" :!type "Object Class Reference"))
      (return (`.bSuccessfullySensed` (break `AIStimulus` _array_element)) _array_element))))

(fn `GetCurrentState`
  (returns (State :type "/Game/BluePrints/Enemy/Enum_AiState Enum"))
  (return (cast `/Game/BluePrints/Enemy/Enum_AiState` (`BlackboardComponent.GetValueAsEnum` (`self.Blackboard`) (`self.stateKeyName`)))))

(fn `HandleSenseSight`
  (params (Actor :type "Actor Object Reference"))
  (bind _state (`self.GetCurrentState`))
  (switch `/Game/BluePrints/Enemy/Enum_AiState` _state
    (:`NewEnumerator0`
      _)
    (:`NewEnumerator3`
      _))
  (if (== Actor (`GameplayStatics.GetPlayerCharacter` 0))
    (`self.SetStateAsAttacking` Actor)))

(fn `HandleSenseSound`
  (params (Location :type "Vector Structure"))
  (bind _state (`self.GetCurrentState`))
  (switch `/Game/BluePrints/Enemy/Enum_AiState` _state
    (:`NewEnumerator0`
      _)
    (:`NewEnumerator3`
      _))
  (`self.SetStateAsInvestigating` Location))

(fn `SetStateAsAttacking`
  (params (AttackTarget :type "Actor Object Reference"))
  (`BlackboardComponent.SetValueAsObject` (`self.Blackboard`) (`self.attackTargetKeyName`) AttackTarget)
  (`BlackboardComponent.SetValueAsEnum` (`self.Blackboard`) (`self.stateKey`) (enumliteral `/Game/BluePrints/Enemy/Enum_AiState` "NewEnumerator1")))

(fn `SetStateAsIdle`
  (`BlackboardComponent.SetValueAsEnum` (`self.Blackboard`) (`self.stateKey`) (enumliteral `/Game/BluePrints/Enemy/Enum_AiState` "NewEnumerator0")))

(fn `SetStateAsInvestigating`
  (params (Location :type "Vector Structure"))
  (`BlackboardComponent.SetValueAsEnum` (`self.Blackboard`) (`self.stateKey`) (enumliteral `/Game/BluePrints/Enemy/Enum_AiState` "NewEnumerator3"))
  (`BlackboardComponent.SetValueAsVector` (`self.Blackboard`) (`self.PointOfInterestKeyName`) Location))

(fn `SetStateAsOnDamaged`
  (`BlackboardComponent.SetValueAsEnum` (`self.Blackboard`) (`self.isHitKey`) (enumliteral `/Game/BluePrints/Enemy/Enum_AiState` "NewEnumerator5")))

(fn `UserConstructionScript`)